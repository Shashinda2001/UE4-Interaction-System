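; BP_Door is an interactable door that swings open and closed.
; Interact checks IsDoorOpen and calls OpenDoor or CloseDoor, each of which updates that flag.
; A single timeline drives the relative yaw of StaticMesh1, playing forward to open and reversing to close.
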(event Custom|OpenDoor
  (Variables|Default|SetisDoorOpen true)
  (bind _doorroatate (Timeline|openDoorTimeLine Play)
    (:Update
      (Transformation|SetRelativeRotation (Variables|Default|GetStaticMesh1) (Math|Rotator|MakeRotator 0.0 0.0 _doorroatate) false false))))

(event Custom|CloseDoor
  (Variables|Default|SetisDoorOpen false)
  (bind _doorroatate (Timeline|openDoorTimeLine Reverse)
    (:Update
      (Transformation|SetRelativeRotation (Variables|Default|GetStaticMesh1) (Math|Rotator|MakeRotator 0.0 0.0 _doorroatate) false false))))

(event EventBeginPlay)

(event EventInteract
  (params (interactActor :type Actor%20Object%20Reference))
  (if (Variables|Default|GetisDoorOpen)
    (CallFunction|CloseDoor)
    (else
      (CallFunction|OpenDoor))))

(fn ConstructionScript)